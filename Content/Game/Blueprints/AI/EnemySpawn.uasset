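; EnemySpawn is a spawner actor that creates EnemyPawns at its own location on a timed schedule.
; Tick accumulates elapsed time, spawns for each SpawnInfomation entry whose AppearanceTime has passed, and removes that entry by index inside the same loop.
; SpawnEnemy spawns even if colliding, creates the default controller, and passes the entry's via points and a Navigation reference to EnemyAI, logging if the cast fails.
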(event EventBeginPlay)

(event Collision|EventActorBeginOverlap
  (params (OtherActor :type Actor%20Object%20Reference)))

(event EventTick
  (params (DeltaSeconds :type Float%20%28single-precision%29))
  (Variables|Default|SetElapsedTime (+ DeltaSeconds (Variables|Default|GetElapsedTime)))
  (for (_array_element _array_index) (Variables|Default|GetSpawnInfomation)
    (if (<= (.appearancetime _array_element) (Variables|Default|GetElapsedTime))
      (CallFunction|SpawnEnemy (Transformation|GetActorLocation) (.viapoints _array_element) (Variables|Default|GetNavigation))
      (Utilities|Array|RemoveIndex (Variables|Default|GetSpawnInfomation) _array_index))))

(fn ConstructionScript)

(fn SpawnEnemy
  (params (Location :type Vector) (TargetActors :type Array%20of%20Actor%20Object%20References) (Navigation :type Navigation%20Volume%20Object%20Reference))
  (bind _returnvalue (Game|SpawnActorfromClass "/Game/Game/Blueprints/Character/EnemyPawn.EnemyPawn_C" (Math|Transform|MakeTransform Location "0, 0, 0" "1,1,1") true 0 0))
  (Pawn|SpawnDefaultController _returnvalue)
  (bind _asenemy_ai (Utilities|Casting|CastToEnemyAI (Pawn|GetController _returnvalue))
    (:then
      (Default|SetTargetActors _asenemy_ai TargetActors)
      (Variables|/Game/Game/Blueprints/AI/CharacterAI/EnemyAI.EnemyAI_C|SetNavigation _asenemy_ai Navigation))
    (:CastFailed
      (Class|VisualLoggerKismetLibrary|LogText "[EnemySpawn : SpawnEnemy] Cast Failed" "Blueprint Log"))))