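; Actor component, judging by its name, that acts as an indexed stopwatch for measuring and printing elapsed time.
; BeginPlay sizes the StartTime and EndTime arrays to CounterCount.
; Start stamps both arrays at an index with Now, and End overwrites only the end time.
; Display prints the index and the millisecond component of the difference via GetMilliseconds, with a Japanese "measured time" label.
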(event EventBeginPlay
  (Utilities|Array|Resize (Variables|Default|GetStartTime) (Variables|処理時間計測|GetCounterCount))
  (Utilities|Array|Resize (Variables|Default|GetEndTime) (Variables|処理時間計測|GetCounterCount)))

(fn Start
  (params (Index :type Integer))
  (bind _returnvalue (Math|DateTime|Now))
  (Utilities|Array|SetArrayElem (Variables|Default|GetStartTime) Index _returnvalue)
  (Utilities|Array|SetArrayElem (Variables|Default|GetEndTime) Index _returnvalue))

(fn End
  (params (Index :type Integer))
  (Utilities|Array|SetArrayElem (Variables|Default|GetEndTime) Index (Math|DateTime|Now)))

(fn Display
  (params (Index :type Integer))
  (Development|PrintString (Utilities|String|BuildString(Integer) (Utilities|String|BuildString(Integer) "" "[" Index "]") "計測時間：" (Class|KismetMathLibrary|GetMilliseconds (- (Utilities|Array|Get(acopy) (Variables|Default|GetEndTime) Index) (Utilities|Array|Get(acopy) (Variables|Default|GetStartTime) Index))) "ms")))